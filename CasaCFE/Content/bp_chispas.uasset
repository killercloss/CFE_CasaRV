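; Sparks effect actor that switches its particle system on or off according to the Activo flag.
; The Activar function activates the particles and sets the flag, so other Blueprints can start the sparks later.
; The construction script calls it when the flag is set.
; BeginPlay does the same and also disables actor tick, or deactivates the particles when the flag is off.
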(event EventBeginPlay
  (if (Variables|Default|GetActivo)
    (CallFunction|Activar)
    (Actor|Tick|SetActorTickEnabled false)
    (else
      (Components|Activation|Deactivate (Variables|Default|GetParticleSystem)))))

(event EventTick
  (params (DeltaSeconds :type Float%20%28single-precision%29)))

(fn ConstructionScript
  (if (Variables|Default|GetActivo)
    (CallFunction|Activar)))

(fn Activar
  (Components|Activation|Activate (Variables|Default|GetParticleSystem) false)
  (Variables|Default|SetActivo true))