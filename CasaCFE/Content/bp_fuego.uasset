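; Fire actor that can start lit or unlit and spreads by heating neighboring fire actors.
; While lit, a Tick throttled by a Delay raises the temperature of unlit fires overlapping its collider by the spread speed, igniting them at a threshold.
; Activar and Desactivar toggle the fire and smoke effects and the active flag.
; Apagar lowers temperature per call, extinguishing the fire at zero.
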(event EventBeginPlay
  (if (Variables|Default|Getactivado)
    (CallFunction|Activar)
    (Actor|Tick|SetActorTickEnabled true)))

(event EventTick
  (params (DeltaSeconds :type Float%20%28single-precision%29))
  (Utilities|FlowControl|Delay 0.2)
  (if (Variables|Default|Getactivado)
    (CallFunction|Propagar)))

(fn ConstructionScript
  (if (Variables|Default|Getactivado)
    (CallFunction|Activar)))

(fn Activar
  (Components|Activation|Activate (Variables|Default|Getfuego) false)
  (Components|Activation|Activate (Variables|Default|Gethumo) false)
  (Variables|Default|Setactivado true))

(fn Propagar
  (for _array_element (Collision|GetOverlappingActors (Variables|Default|Getcollider) "bp_fuego_C" :!class /Script/Engine.PrimitiveComponent)
    (bind _asbp_fuego (Utilities|Casting|CastTobp_fuego _array_element))
    (if (not (Variables|bp_fuego_C|Getactivado _asbp_fuego))
      (bind _output_get (Variables|bp_fuego_C|Settemperatura _asbp_fuego (+ (Variables|bp_fuego_C|Gettemperatura _asbp_fuego) (Variables|Default|Getvelocidad%20del%20fuego))))
      (if (>= _output_get (Variables|Default|Gettemperatura%20limite))
        (CallFunction|Activar _asbp_fuego)))))

(fn Desactivar
  (Components|Activation|Deactivate (Variables|Default|Getfuego))
  (Components|Activation|Deactivate (Variables|Default|Gethumo))
  (Variables|Default|Setactivado false))

(fn Apagar
  (params (distancia :type Float%20%28single-precision%29))
  (Variables|Default|Settemperatura (- (Variables|Default|Gettemperatura) 5))
  (if (not (> (Variables|Default|Gettemperatura) 0))
    (CallFunction|Desactivar)
    (Variables|Default|Settemperatura 0)
    (Rendering|SetVisibility (Variables|Default|GetTextRender) false false)))